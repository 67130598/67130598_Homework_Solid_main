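; Base Blueprint for interactable actors, supplying default responses for an interaction system.
; It exposes an availability check from the inverse of IsInteract, prompt text built from the display name, and a prompt location at the actor's position.
; OnInteract sets IsInteract to false, so interaction stays available afterward, and prints the object's name as placeholder feedback.
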(event `/Game/Bluprint/Interface/BPI_Interactable.OnInteract`
  (params (Interactor :type "/Game/Bluprint/ThirdPerson/Blueprints/BP_Player_Character Object Reference"))
  (`|ExecutionSequence`
    (:`then_0`
      (set `self.IsInteract` false))
    (:`then_1`
      (`KismetSystemLibrary.PrintText` (`|FormatText` "Interact :{Object}" (`KismetSystemLibrary.GetObjectName` self))))))

(fn `CanInteractable`
  (returns (`Return Is Can` :type Boolean))
  (return (not (`self.IsInteract`))))

(fn `GetInteractText`
  (returns (`Return Text` :type Text))
  (return (`|FormatText` "Interact at : {Object}" (`KismetSystemLibrary.GetDisplayName` self))))

(fn `GetInteractTextLocation`
  (returns (ReturnVector :type "Vector Structure"))
  (return (`self.K2_GetActorLocation`)))

(fn `UserConstructionScript`)