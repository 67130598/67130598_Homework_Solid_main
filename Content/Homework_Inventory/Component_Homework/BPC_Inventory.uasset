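; Inventory component that stores stackable items in a map from item class to a single constructed instance holding its Quantity.
; Adding increments the stack or constructs a new instance, then fires OnInventoryUpdated.
; Using an item, looked up by class despite the UseItemBySlot name, sends a Consume interface message with the user and decrements Quantity, without firing the update or removing empty entries.
; A count query returns Quantity, or zero when absent.
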(event `self.ReceiveBeginPlay`)

(event `UpdateUI`)

(event `self.ReceiveTick`
  (params (DeltaSeconds :type "Float (single-precision)")))

(fn `AddItemByClass`
  (params (ItemClass :type "/Game/Homework_Inventory/InventoryData/BP_InventoryItem_Base Class Reference"))
  (bind (_value _returnvalue) (`BlueprintMapLibrary.Map_Find` (`self.InventoryLis`) ItemClass))
  (if _returnvalue
    (set `/Game/Homework_Inventory/InventoryData/BP_InventoryItem_Base.Quantity` (+ (`/Game/Homework_Inventory/InventoryData/BP_InventoryItem_Base.Quantity` _value) 1) _value)
    (else
      (bind _returnvalue_2 (`|GenericCreateObject` self ItemClass))
      (set `/Game/Homework_Inventory/InventoryData/BP_InventoryItem_Base.Quantity` 1 _returnvalue_2)
      (`BlueprintMapLibrary.Map_Add` (`self.InventoryLis`) ItemClass _returnvalue_2)))
  (`self.OnInventoryUpdated`))

(fn `GetItemCount`
  (params (ItemClass :type "/Game/Homework_Inventory/InventoryData/BP_InventoryItem_Base Class Reference"))
  (returns (Count :type Integer))
  (bind (_value _returnvalue) (`BlueprintMapLibrary.Map_Find` (`self.InventoryLis`) ItemClass))
  (if _returnvalue
    (return (`/Game/Homework_Inventory/InventoryData/BP_InventoryItem_Base.Quantity` _value))
    (else
      (return 0))))

(fn `UseItemBySlot`
  (params (ItemClass :type "/Game/Homework_Inventory/InventoryData/BP_InventoryItem_Base Class Reference") (User :type "/Game/Bluprint/ThirdPerson/Blueprints/BP_Player_Character Object Reference"))
  (bind (_value _returnvalue) (`BlueprintMapLibrary.Map_Find` (`self.InventoryLis`) ItemClass))
  (if _returnvalue
    (if (> (`/Game/Homework_Inventory/InventoryData/BP_InventoryItem_Base.Quantity` _value) 0)
      (message `/Game/Homework_Inventory/InventoryData/BPI_ConsumeItemable.Consume` _value User)
      (set `/Game/Homework_Inventory/InventoryData/BP_InventoryItem_Base.Quantity` (- (`/Game/Homework_Inventory/InventoryData/BP_InventoryItem_Base.Quantity` _value) 1) _value))))