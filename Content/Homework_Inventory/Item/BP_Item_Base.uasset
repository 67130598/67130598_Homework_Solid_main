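; BP_Item_Base is an interactable pickup actor that shows "Collect Item" and gives an item to whoever interacts with it.
; On interact, it sets a motion warp target at a short offset toward the interactor, facing the item, then plays a button-press montage on the interactor.
; The montage's "get" notify adds ItemToGiveClass to the interactor's inventory component and destroys the item.
; Montage completion or interruption clears IsInteract.
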(event `/Game/Bluprint/Interface/BPI_Interactable.Oninteract`
  (params (Interactor :type "/Game/Bluprint/ThirdPerson/Blueprints/BP_Player_Character Object Reference"))
  (bind _returnvalue (`self.K2_GetActorLocation` self))
  (bind _returnvalue_2 (`KismetMathLibrary.Normal` (- (`self.K2_GetActorLocation` Interactor) _returnvalue)))
  (`parent.OnInteract` Interactor)
  (`MotionWarpingComponent.AddOrUpdateWarpTargetFromLocationAndRotation` (`/Game/Bluprint/ThirdPerson/Blueprints/BP_ThirdPersonCharacter.MotionWarping` Interactor) "InteractTarget" (+ (* _returnvalue_2 65.0) _returnvalue) (`KismetMathLibrary.MakeRotFromX` (`KismetMathLibrary.MakeVector` (.x (* _returnvalue_2 -1.0)) (.y (* _returnvalue_2 -1.0)))))
  (bind _notifyname (`|PlayMontage` (`Character.Mesh` Interactor) "/Game/Asset/Animations/AM_Press_Button.AM_Press_Button")
    (:`OnCompleted`
      (set `self.IsInteract` false :!label _label))
    (:`OnInterrupted`
      (goto _label))
    (:`OnNotifyBegin`
      (if (== _notifyname "get")
        (`/Game/Homework_Inventory/Component_Homework/BPC_Inventory.AddItemByClass` (`/Game/Bluprint/ThirdPerson/Blueprints/BP_Player_Character.BPC_Inventory` Interactor) (`self.ItemToGiveClass`))
        (`self.K2_DestroyActor`)))))

(fn `GetInteractText`
  (returns (`Return Text` :type Text))
  (return "Collect Item"))

(fn `UserConstructionScript`
  (`parent.UserConstructionScript`))